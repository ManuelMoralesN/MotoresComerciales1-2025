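; BP_Projectile is a projectile actor that flies forward from where it spawns and bursts on tagged obstacles.
; On BeginPlay it sets its ProjectileMovement velocity along the actor's forward vector at a fixed speed.
; When it overlaps an actor tagged ColliderProjectile, it spawns a Niagara effect and a sound at its location, then destroys itself.
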(event EventBeginPlay
  (Variables|/Script/Engine.MovementComponent|SetVelocity (Variables|Default|GetProjectileMovement) (* (Transformation|GetActorForwardVector) 700)))

(event Collision|EventActorBeginOverlap
  (params (OtherActor :type Actor%20Object%20Reference))
  (if (Actor|ActorHasTag OtherActor "ColliderProjectile")
    (Niagara|SpawnSystematLocation "/Game/Resources/NewNiagaraSystem1.NewNiagaraSystem1" (Transformation|GetActorLocation))
    (Audio|SpawnSoundatLocation 0 (Transformation|GetActorLocation) "0, 0, 0" 1.0 1.0 0.0 0 0)
    (Actor|DestroyActor)))

(event EventTick
  (params (DeltaSeconds :type Float%20%28single-precision%29)))

(fn ConstructionScript)